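; BP_SpawnHandler spawns monster encounters when the yellow card and final card pickup events fire.
; Each event spawns a BP_AISpawner and a BP_EventSpawner at their own transforms, then plays a spook or door sound at the first monster location.
; The first event spawner receives its AI spawner through GetSpawner.
; The final-card branch clears BPEventSpawn before calling GetSpawner, so its new event spawner never receives the second spawner.
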(event `self.ReceiveBeginPlay`)

(event `YellowCardWasPickedUp`
  (bind _monsterspawnlocation_location (`KismetMathLibrary.BreakTransform` (`self.MonsterSpawnLocation`)))
  (bind _returnvalue (`|SpawnActorFromClass` "/Game/AI/BP_AISpawner.BP_AISpawner_C" (`self.MonsterSpawnLocation`) "Undefined" "OverrideRootScale" null null))
  (set `self.FirstSpawner` _returnvalue)
  (bind _returnvalue_2 (`|SpawnActorFromClass` "/Game/AI/BP_EventSpawner.BP_EventSpawner_C" (`self.BoxOverlapLocation`) "Undefined" "OverrideRootScale" null null))
  (bind _output_get (set `self.BP_EventSpawn` _returnvalue_2))
  (`/Game/AI/BP_EventSpawner.GetSpawner` _output_get (`self.FirstSpawner`))
  (`GameplayStatics.SpawnSoundAtLocation` "/Game/SFX/spookFixed.spookFixed" _monsterspawnlocation_location (struct) 1.0 1.0 0.0 "/Game/SFX/ATT_Default.ATT_Default" null))

(event `FinalCardPickedUp`
  (bind _monsterspawnlocation_location (`KismetMathLibrary.BreakTransform` (`self.MonsterSpawnLocation`)))
  (bind _returnvalue (`|SpawnActorFromClass` "/Game/AI/BP_AISpawner.BP_AISpawner_C" (`self.MonsterSpawnLocation_02`) "Undefined" "OverrideRootScale" null null))
  (set `self.SecondSpawner` _returnvalue)
  (`|SpawnActorFromClass` "/Game/AI/BP_EventSpawner.BP_EventSpawner_C" (`self.BoxOverlapLocation002`) "Undefined" "OverrideRootScale" null null)
  (bind _output_get (set `self.BP_EventSpawn` null))
  (`/Game/AI/BP_EventSpawner.GetSpawner` _output_get (`self.SecondSpawner`))
  (`GameplayStatics.SpawnSoundAtLocation` "/Game/BlockingStarterPack/Sounds/SimpleDoor_StarClosing01.SimpleDoor_StarClosing01" _monsterspawnlocation_location (struct) 1.0 1.0 0.0 "/Game/BlockingStarterPack/Sounds/DoorSoundAttenuation.DoorSoundAttenuation" null))